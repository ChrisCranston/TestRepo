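; Interactive lift Blueprint, despite its SlideDoors name, that moves a platform mesh between start and end locations.
; Overlapping the button collider plays the MovingUpDown timeline, whose alpha lerps the platform's relative location, and ending the overlap reverses it.
; A Moving flag, set on timeline update and cleared on finish, ignores both overlap events mid-travel, so leaving during movement does not send the platform back.
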(event OnComponentBeginOverlap(LiftButtonCollider)
  (params (OverlappedComponent :type Primitive%20Component%20Object%20Reference) (OtherActor :type Actor%20Object%20Reference) (OtherComp :type Primitive%20Component%20Object%20Reference) (OtherBodyIndex :type Integer) (bFromSweep :type Boolean) (SweepResult :type Hit%20Result%20Structure%20%28by%20ref%29))
  ;[1 1 1] LiftMainFunctionality
  (if (not (Variables|Default|GetMoving?))
    (bind _alpha (Timeline|Moving%20Up/Down Play)
      (:Update
        (Variables|Default|SetMoving? true)
        (Transformation|SetRelativeLocation (Variables|Default|GetLiftPlatformMesh) (Math|Vector|Lerp(Vector) (Variables|Default|GetStartLocation) (Variables|Default|GetEndLocation) _alpha) false false))
      (:Finished
        (Variables|Default|SetMoving? false)))))

(event OnComponentEndOverlap(LiftButtonCollider)
  (params (OverlappedComponent :type Primitive%20Component%20Object%20Reference) (OtherActor :type Actor%20Object%20Reference) (OtherComp :type Primitive%20Component%20Object%20Reference) (OtherBodyIndex :type Integer))
  ;[1 1 1] LiftMainFunctionality
  (if (not (Variables|Default|GetMoving?))
    (bind _alpha (Timeline|Moving%20Up/Down Reverse)
      (:Update
        (Variables|Default|SetMoving? true)
        (Transformation|SetRelativeLocation (Variables|Default|GetLiftPlatformMesh) (Math|Vector|Lerp(Vector) (Variables|Default|GetStartLocation) (Variables|Default|GetEndLocation) _alpha) false false))
      (:Finished
        (Variables|Default|SetMoving? false)))))

(fn ConstructionScript)