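; BP_Lift is an interactive lift whose platform moves between a start and end location when the player presses E.
; Overlapping the button collider as ThirdPersonCharacter enables input and shows a hint widget; leaving reverses both.
; The MovingUpDown timeline lerps the platform, playing or reversing by IsOnTop, with a Moving guard and a state flip on finish.
; GetLift triggers the same toggle without a key press, while CallLift is a stub returning false.
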(event OnComponentBeginOverlap(LiftButtonCollider)
  (params (OverlappedComponent :type Primitive%20Component%20Object%20Reference) (OtherActor :type Actor%20Object%20Reference) (OtherComp :type Primitive%20Component%20Object%20Reference) (OtherBodyIndex :type Integer) (bFromSweep :type Boolean) (SweepResult :type Hit%20Result%20Structure%20%28by%20ref%29))
  ;[1 1 1] Overlay for Input
  (Utilities|Casting|CastToThirdPersonCharacter OtherActor)
  (Input|EnableInput (Game|GetPlayerController 0))
  (CallFunction|ShowHint))

(event OnComponentEndOverlap(LiftButtonCollider)
  (params (OverlappedComponent :type Primitive%20Component%20Object%20Reference) (OtherActor :type Actor%20Object%20Reference) (OtherComp :type Primitive%20Component%20Object%20Reference) (OtherBodyIndex :type Integer))
  ;[1 1 1] Overlay for Input
  (Utilities|Casting|CastToThirdPersonCharacter OtherActor)
  (Input|DisableInput (Game|GetPlayerController 0))
  (CallFunction|RemoveHint))

(event Custom|GetLift
  ;[1 1 1] LiftMainFunctionality
  (if (Variables|Default|GetIsOnTop)
    (if (not (Variables|Default|GetMoving?))
      (bind _alpha (Timeline|Moving%20Up/Down Reverse)
        (:Update
          (Variables|Default|SetMoving? true)
          (Transformation|SetRelativeLocation (Variables|Default|GetLiftPlatformMesh) (Math|Vector|Lerp(Vector) (Variables|Default|GetStartLocation) (Variables|Default|GetEndLocation) _alpha) false false))
        (:Finished
          (Variables|Default|SetMoving? false)
          (CallFunction|SetTop/Bot))))
    (elif (not (Variables|Default|GetMoving?))
      (Timeline|Moving%20Up/Down Play))))

(event Input|KeyboardEvents|E
  (params (Key :type Key%20Structure :default "None"))
  ;[1 1 1] LiftMainFunctionality
  (:Pressed
    (if (Variables|Default|GetIsOnTop)
      (if (not (Variables|Default|GetMoving?))
        (bind _alpha (Timeline|Moving%20Up/Down Reverse)
          (:Update
            (Variables|Default|SetMoving? true)
            (Transformation|SetRelativeLocation (Variables|Default|GetLiftPlatformMesh) (Math|Vector|Lerp(Vector) (Variables|Default|GetStartLocation) (Variables|Default|GetEndLocation) _alpha) false false))
          (:Finished
            (Variables|Default|SetMoving? false)
            (CallFunction|SetTop/Bot))))
      (elif (not (Variables|Default|GetMoving?))
        (Timeline|Moving%20Up/Down Play)))))

(fn ConstructionScript)

(fn ShowHint
  (bind _returnvalue (UserInterface|CreateWidget (Variables|Default|GetLiftHintWidget)))
  (bind _output_get (Variables|Default|SetLiftHintWidgetReferences _returnvalue))
  (UserInterface|Viewport|AddtoViewport _output_get 0))

(fn RemoveHint
  (Widget|RemovefromParent (Variables|Default|GetLiftHintWidgetReferences)))

(fn SetTop/Bot
  (if (Variables|Default|GetIsOnTop)
    (Variables|Default|SetIsOnTop false)
    (else
      (Variables|Default|SetIsOnTop true))))

(fn CallLift
  (return false))