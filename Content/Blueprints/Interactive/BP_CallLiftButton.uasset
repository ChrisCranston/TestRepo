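; An interactive lift call button that lets the player summon a referenced lift.
; When a ThirdPersonCharacter enters its box, it enables input for the first player controller, shows a LiftHintWidget and prints a debug string.
; Pressing E then calls GetLift on the MyLift reference.
; Leaving the box disables input and removes the hint from the screen.
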(event OnComponentBeginOverlap(Box)
  (params (OverlappedComponent :type Primitive%20Component%20Object%20Reference) (OtherActor :type Actor%20Object%20Reference) (OtherComp :type Primitive%20Component%20Object%20Reference) (OtherBodyIndex :type Integer) (bFromSweep :type Boolean) (SweepResult :type Hit%20Result%20Structure%20%28by%20ref%29))
  ;[1 1 1] Overlay for input
  (Utilities|Casting|CastToThirdPersonCharacter OtherActor)
  (Input|EnableInput (Game|GetPlayerController 0))
  (CallFunction|CreateHint)
  (Development|PrintString "Hello"))

(event OnComponentEndOverlap(Box)
  (params (OverlappedComponent :type Primitive%20Component%20Object%20Reference) (OtherActor :type Actor%20Object%20Reference) (OtherComp :type Primitive%20Component%20Object%20Reference) (OtherBodyIndex :type Integer))
  ;[1 1 1] Overlay for input
  (Utilities|Casting|CastToThirdPersonCharacter OtherActor)
  (Input|DisableInput (Game|GetPlayerController 0))
  (CallFunction|RemoveHint))

(event Input|KeyboardEvents|E
  (params (Key :type Key%20Structure :default "None"))
  (:Pressed
    (Default|GetLift (Variables|Default|GetMyLift))))

(fn ConstructionScript)

(fn CreateHint
  (bind _returnvalue (UserInterface|CreateWidget (Variables|Default|GetLiftHintWidget)))
  (bind _output_get (Variables|Default|SetHintWidgetReferences _returnvalue))
  (UserInterface|Viewport|AddtoViewport _output_get 0))

(fn RemoveHint
  (Widget|RemovefromParent (Variables|Default|GetHintWidgetReferences)))